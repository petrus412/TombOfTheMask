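; BP_SoundManager is an actor that plays one-shot sound cues for point pickups, player movement, stops and death.
; On BeginPlay it binds to the destroyed event of every BP_Points actor and to the Move, SoundStop and Death dispatchers on BP_PlayerController.
; Each handler plays its own cue at the player pawn's location, so gameplay classes only broadcast events and hold no audio logic for these sounds.
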(event Custom|Collected
  (Audio|PlaySoundatLocation "/Game/Blueprints/Sound/Cue/Bing_F_Cue.Bing_F_Cue" (Transformation|GetActorLocation (Game|Player|GetPlayerPawn 0)) "0, 0, 0" 1.0 1.0 0.0 0 0 0))

(event Custom|Stop
  (Audio|PlaySoundatLocation "/Game/Blueprints/Sound/Cue/Bop_Cue.Bop_Cue" (Transformation|GetActorLocation (Game|Player|GetPlayerPawn 0)) "0, 0, 0" 1.0 1.0 0.0 0 0 0))

(event Custom|Move
  (Audio|PlaySoundatLocation "/Game/Blueprints/Sound/Cue/Untitled_Cue.Untitled_Cue" (Transformation|GetActorLocation (Game|Player|GetPlayerPawn 0)) "0, 0, 0" 1.0 1.0 0.0 0 0 0))

(event Custom|Death
  (Audio|PlaySoundatLocation "/Game/Blueprints/Sound/Cue/Bavk_You_Cue.Bavk_You_Cue" (Transformation|GetActorLocation (Game|Player|GetPlayerPawn 0)) "0, 0, 0" 1.0 1.0 0.0 0 0 0))

(event EventBeginPlay
  (bind _outactors (Actor|GetAllActorsOfClass "/Game/Blueprints/Actor/Collectable/BP_Points.BP_Points_C"))
  (for _array_element _outactors
    (EventDispatchers|BindEventtoDestroyed _array_element (delegate Custom|Collected)))
  (bind _asbp_player_controller (Utilities|Casting|CastToBP_PlayerController (Game|GetPlayerController 0)))
  (EventDispatchers|BindEventtoSoundStop _asbp_player_controller (delegate Custom|Stop))
  (EventDispatchers|BindEventtoMove _asbp_player_controller (delegate Custom|Move))
  (EventDispatchers|BindEventtoDeath _asbp_player_controller (delegate Custom|Death)))

(fn ConstructionScript)