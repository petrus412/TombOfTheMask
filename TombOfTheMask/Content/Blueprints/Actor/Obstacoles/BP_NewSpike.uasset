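; BP_NewSpike is a short-lived spike obstacle that makes the player lose when it touches the BP_Mask character.
; On BeginPlay it jumps instantly along its own up vector, so the offset follows its rotation, then destroys itself after a brief delay.
; Its Box overlap filters for BP_Mask and calls Lose on the first player's BP_PlayerController.
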(event OnComponentBeginOverlap(Box)
  (params (OverlappedComponent :type Primitive%20Component%20Object%20Reference) (OtherActor :type Actor%20Object%20Reference) (OtherComp :type Primitive%20Component%20Object%20Reference) (OtherBodyIndex :type Integer) (bFromSweep :type Boolean) (SweepResult :type Hit%20Result%20Structure%20%28by%20ref%29))
  (Utilities|Casting|CastToBP_Mask OtherActor)
  (bind _asbp_player_controller (Utilities|Casting|CastToBP_PlayerController (Game|GetPlayerController 0)))
  (Default|Lose _asbp_player_controller))

(event EventBeginPlay
  (Variables|Default|SetPosition (Transformation|GetActorLocation))
  (Transformation|SetActorLocation (+ (* (Math|Vector|GetUpVector (Transformation|GetActorRotation)) 5e+01) (Variables|Default|GetPosition)) false false)
  (Utilities|FlowControl|Delay 0.5)
  (Actor|DestroyActor))

(fn ConstructionScript)