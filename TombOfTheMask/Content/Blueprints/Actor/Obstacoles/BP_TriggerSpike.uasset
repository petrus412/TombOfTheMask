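; Obstacle actor with a spike on each of four sides (front, back, left, right) that makes the player's BP_Mask lose.
; When the mask enters a side's trigger box, that spike moves out after a half-second delay and retracts half a second later.
; CallLose fires if the mask is in that side's death box as the spike extends, or enters it while the side's Out flag is set.
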(event OnComponentBeginOverlap(FrontDeathBox)
  (params (OverlappedComponent :type Primitive%20Component%20Object%20Reference) (OtherActor :type Actor%20Object%20Reference) (OtherComp :type Primitive%20Component%20Object%20Reference) (OtherBodyIndex :type Integer) (bFromSweep :type Boolean) (SweepResult :type Hit%20Result%20Structure%20%28by%20ref%29))
  (if (Variables|Default|GetOutFront)
    (Utilities|Casting|CastToBP_Mask OtherActor)
    (Default|CallLose)))

(event OnComponentBeginOverlap(BackDeathBox)
  (params (OverlappedComponent :type Primitive%20Component%20Object%20Reference) (OtherActor :type Actor%20Object%20Reference) (OtherComp :type Primitive%20Component%20Object%20Reference) (OtherBodyIndex :type Integer) (bFromSweep :type Boolean) (SweepResult :type Hit%20Result%20Structure%20%28by%20ref%29))
  (if (Variables|Default|GetOutBack)
    (Utilities|Casting|CastToBP_Mask OtherActor)
    (Default|CallLose)))

(event OnComponentBeginOverlap(LeftDeathBox)
  (params (OverlappedComponent :type Primitive%20Component%20Object%20Reference) (OtherActor :type Actor%20Object%20Reference) (OtherComp :type Primitive%20Component%20Object%20Reference) (OtherBodyIndex :type Integer) (bFromSweep :type Boolean) (SweepResult :type Hit%20Result%20Structure%20%28by%20ref%29))
  (if (Variables|Default|GetOutLeft)
    (Utilities|Casting|CastToBP_Mask OtherActor)
    (Default|CallLose)))

(event OnComponentBeginOverlap(RightDeathBox)
  (params (OverlappedComponent :type Primitive%20Component%20Object%20Reference) (OtherActor :type Actor%20Object%20Reference) (OtherComp :type Primitive%20Component%20Object%20Reference) (OtherBodyIndex :type Integer) (bFromSweep :type Boolean) (SweepResult :type Hit%20Result%20Structure%20%28by%20ref%29))
  (if (Variables|Default|GetOutRight)
    (Utilities|Casting|CastToBP_Mask OtherActor)
    (Default|CallLose)))

(event OnComponentBeginOverlap(BoxFront)
  (params (OverlappedComponent :type Primitive%20Component%20Object%20Reference) (OtherActor :type Actor%20Object%20Reference) (OtherComp :type Primitive%20Component%20Object%20Reference) (OtherBodyIndex :type Integer) (bFromSweep :type Boolean) (SweepResult :type Hit%20Result%20Structure%20%28by%20ref%29))
  (bind _front_spike (Variables|Default|GetFront%20Spike))
  (Utilities|Casting|CastToBP_Mask OtherActor)
  (Utilities|FlowControl|Delay 0.5)
  (Transformation|SetRelativeLocation _front_spike "-1.000000, 0, 0" false false)
  (Variables|Default|SetOutFront true)
  (if (Collision|IsOverlappingActor (Variables|Default|GetFront%20DeathBox) (Variables|Default|GetMask) :!class /Script/Engine.PrimitiveComponent)
    (Default|CallLose))
  (Utilities|FlowControl|Delay 0.5)
  (Transformation|SetRelativeLocation _front_spike "-101.000000, 0, 0" false false)
  (Variables|Default|SetOutFront false))

(event OnComponentBeginOverlap(BoxBack)
  (params (OverlappedComponent :type Primitive%20Component%20Object%20Reference) (OtherActor :type Actor%20Object%20Reference) (OtherComp :type Primitive%20Component%20Object%20Reference) (OtherBodyIndex :type Integer) (bFromSweep :type Boolean) (SweepResult :type Hit%20Result%20Structure%20%28by%20ref%29))
  (bind _back_spike (Variables|Default|GetBack%20Spike))
  (Utilities|Casting|CastToBP_Mask OtherActor)
  (Utilities|FlowControl|Delay 0.5)
  (Transformation|SetRelativeLocation _back_spike "1.000000, 0,0.000000" false false)
  (Variables|Default|SetOutBack true)
  (if (Collision|IsOverlappingActor (Variables|Default|GetBack%20DeathBox) (Variables|Default|GetMask) :!class /Script/Engine.PrimitiveComponent)
    (Default|CallLose))
  (Utilities|FlowControl|Delay 0.5)
  (Transformation|SetRelativeLocation _back_spike "101.000000, 0, 0" false false)
  (Variables|Default|SetOutBack false))

(event OnComponentBeginOverlap(BoxLeft)
  (params (OverlappedComponent :type Primitive%20Component%20Object%20Reference) (OtherActor :type Actor%20Object%20Reference) (OtherComp :type Primitive%20Component%20Object%20Reference) (OtherBodyIndex :type Integer) (bFromSweep :type Boolean) (SweepResult :type Hit%20Result%20Structure%20%28by%20ref%29))
  (bind _left_spike (Variables|Default|GetLeft%20Spike))
  (Utilities|Casting|CastToBP_Mask OtherActor)
  (Utilities|FlowControl|Delay 0.5)
  (Transformation|SetRelativeLocation _left_spike "0.000000,-1.000000, 0" false false)
  (Variables|Default|SetOutLeft true)
  (if (Collision|IsOverlappingActor (Variables|Default|GetLeft%20DeathBox) (Variables|Default|GetMask) :!class /Script/Engine.PrimitiveComponent)
    (Default|CallLose))
  (Utilities|FlowControl|Delay 0.5)
  (Transformation|SetRelativeLocation _left_spike "0.000000,-101.000000, 0" false false)
  (Variables|Default|SetOutLeft false))

(event OnComponentBeginOverlap(BoxRight)
  (params (OverlappedComponent :type Primitive%20Component%20Object%20Reference) (OtherActor :type Actor%20Object%20Reference) (OtherComp :type Primitive%20Component%20Object%20Reference) (OtherBodyIndex :type Integer) (bFromSweep :type Boolean) (SweepResult :type Hit%20Result%20Structure%20%28by%20ref%29))
  (bind _right_spike (Variables|Default|GetRight%20Spike))
  (Utilities|Casting|CastToBP_Mask OtherActor)
  (Utilities|FlowControl|Delay 0.5)
  (Transformation|SetRelativeLocation _right_spike "0.000000,1.000000, 0" false false)
  (Variables|Default|SetOutRight true)
  (if (Collision|IsOverlappingActor (Variables|Default|GetRight%20DeathBox) (Variables|Default|GetMask) :!class /Script/Engine.PrimitiveComponent)
    (Default|CallLose))
  (Utilities|FlowControl|Delay 0.5)
  (Transformation|SetRelativeLocation _right_spike "0.000000,101.000000, 0" false false)
  (Variables|Default|SetOutRight false))

(event EventBeginPlay
  (bind _asbp_mask (Utilities|Casting|CastToBP_Mask (Game|Player|GetPlayerPawn 0)))
  (Variables|Default|SetMask _asbp_mask))

(fn ConstructionScript)