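; BP_Bat is a moving obstacle that triggers a loss by bat when its Box overlaps a BP_Mask.
; From BeginPlay, Timeline_1 lerps it one Tile offset at a time along Y or X, chosen by Direction, without sweeping.
; Each finished timeline loops into the next step; after Total steps it resets the counter, modifies Tile, apparently to reverse travel, and briefly pauses before continuing.
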(event OnComponentBeginOverlap(Box)
  (params (OverlappedComponent :type Primitive%20Component%20Object%20Reference) (OtherActor :type Actor%20Object%20Reference) (OtherComp :type Primitive%20Component%20Object%20Reference) (OtherBodyIndex :type Integer) (bFromSweep :type Boolean) (SweepResult :type Hit%20Result%20Structure%20%28by%20ref%29))
  (Utilities|Casting|CastToBP_Mask OtherActor)
  (Default|CallLosebyBat))

(event EventBeginPlay
  (bind _returnvalue (Transformation|GetActorLocation))
  (bind _returnvalue_2 (Transformation|GetActorLocation))
  (bind _tile (Variables|Default|GetTile))
  (if (Variables|Default|Getdirection) :!label _label
    (Variables|Default|SetStartPosition (.y _returnvalue_2))
    (Variables|Default|SetEndPosition (+ (.y _returnvalue_2) _tile))
    (bind _movement (Timeline|Timeline_1 PlayFromStart)
      (:Update
        (if (Variables|Default|Getdirection)
          (Variables|Default|Settest (Math|Vector|MakeVector (.x _returnvalue) (Math|Float|Lerp (Variables|Default|GetStartPosition) (Variables|Default|GetEndPosition) _movement) (.z _returnvalue)))
          (else
            (Variables|Default|Settest (Math|Vector|MakeVector (Math|Float|Lerp (Variables|Default|GetStartPosition) (Variables|Default|GetEndPosition) _movement) (.y _returnvalue) (.z _returnvalue)))))
        (Transformation|SetActorLocation (Variables|Default|Gettest) false false))
      (:Finished
        (bind _result (Math|Integer|IncrementInt (Variables|Default|Getmove))
          (:%20%20
            (if (== _result (Variables|Default|GetTotal))
              (Variables|Default|Setmove 0)
              (Math|Float|NegateFloat (Variables|Default|GetTile)
                (:%20%20
                  (Utilities|FlowControl|Delay 0.4)
                  (goto _label)))
              (else
                (goto _label)))))))
    (else
      (Variables|Default|SetStartPosition (.x _returnvalue_2))
      (Variables|Default|SetEndPosition (+ (.x _returnvalue_2) _tile))
      (Timeline|Timeline_1 PlayFromStart))))

(fn ConstructionScript)

(fn Check
  (return))