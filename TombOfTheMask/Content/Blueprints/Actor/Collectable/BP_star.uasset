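; BP_star is a collectable star actor that counts toward the player's total when a BP_Mask actor overlaps it.
; On overlap it applies a force to its Destructible component at the actor's location.
; A boolean guard lets it increment the Starts counter on BP_PlayerController only once, then the star destroys itself after a short delay.
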(event Collision|EventActorBeginOverlap
  (params (OtherActor :type Actor%20Object%20Reference))
  (Utilities|Casting|CastToBP_Mask OtherActor)
  (Class|PrimitiveComponent|AddForceatLocation (Variables|Default|GetDestructible) "100.000000,100.000000, 0" (Transformation|GetActorLocation) "None")
  (bind _asbp_player_controller (Utilities|Casting|CastToBP_PlayerController (Game|GetPlayerController 0)))
  (if (Variables|Default|Get+)
    (Variables|Default|Set+ false)
    (Math|Integer|IncrementInt (Variables|/Game/Blueprints/Pawn/BP_PlayerController.BP_PlayerController_C|GetStarts _asbp_player_controller)
      (:%20%20
        (Utilities|FlowControl|Delay 1.0)
        (Actor|DestroyActor)))))

(fn ConstructionScript)