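; Player controller for a four-level sliding game in which a mask pawn travels in straight lines until it hits a wall, collecting points and avoiding spikes and bats.
; Directional input checks adjacent tagged walls before starting a move, Tick translates the mask with trail effects, and pawn hit events snap it beside the obstacle.
; BeginPlay binds point, hazard and level-end events, driving scoring, shatter-on-death and per-level saving to the BP_Var game instance.
; It also handles pause, restart and return-to-menu input.
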(event Custom|Stop%20Front
  (params (hitted :type Actor%20Object%20Reference))
  (bind _returnvalue (Transformation|GetActorLocation hitted))
  ;[1 1 1] Hit Front
  (if (== (Variables|Default|GetDirection) 0)
    (Variables|Default|Setmoving false)
    (Variables|Default|SetPosition (Math|Vector|MakeVector (- (.x _returnvalue) 1e+02) (.y _returnvalue) 5e+01))
    (Transformation|SetActorLocation (Variables|Default|GetMask) (Variables|Default|GetPosition) false false)
    (Variables|Default|SetEmitter%20position (Math|Vector|MakeVector (+ (.X (Math|Vector|BreakVector (Variables|Default|GetPosition))) 4e+01) (.Y (Math|Vector|BreakVector (Variables|Default|GetPosition))) (.Z (Math|Vector|BreakVector (Variables|Default|GetPosition)))))
    (Variables|Default|Setemitter%20rotation "0.000000,90.000000,90.000000")
    ;[1 1 1] Play end movment effect
    (Effects|SpawnEmitteratLocation "/Game/Cascade/Hit.Hit" (Variables|Default|GetEmitter%20position) (Variables|Default|Getemitter%20rotation))
    (Components|StaticMesh|SetStaticMesh (Variables|/Game/Blueprints/Pawn/BP_Mask.BP_Mask_C|GetStaticMesh (Variables|Default|GetMask)) "/Game/SaticMesh/maschera.maschera")
    (Default|CallSoundStop)))

(event Custom|Stop%20Back
  (params (hitted :type Actor%20Object%20Reference))
  (bind _returnvalue (Transformation|GetActorLocation hitted))
  ;[1 1 1] Hit Back
  (if (== (Variables|Default|GetDirection) 1)
    (Variables|Default|Setmoving false)
    (Variables|Default|SetPosition (Math|Vector|MakeVector (- (.x _returnvalue) -1e+02) (.y _returnvalue) 5e+01))
    (Transformation|SetActorLocation (Variables|Default|GetMask) (Variables|Default|GetPosition) false false)
    (Variables|Default|SetEmitter%20position (Math|Vector|MakeVector (+ (.X (Math|Vector|BreakVector (Variables|Default|GetPosition))) -4e+01) (.Y (Math|Vector|BreakVector (Variables|Default|GetPosition))) (.Z (Math|Vector|BreakVector (Variables|Default|GetPosition)))))
    (Variables|Default|Setemitter%20rotation "0.000000,-90.000000,90.000000")
    ;[1 1 1] Play end movment effect
    (Effects|SpawnEmitteratLocation "/Game/Cascade/Hit.Hit" (Variables|Default|GetEmitter%20position) (Variables|Default|Getemitter%20rotation))
    (Components|StaticMesh|SetStaticMesh (Variables|/Game/Blueprints/Pawn/BP_Mask.BP_Mask_C|GetStaticMesh (Variables|Default|GetMask)) "/Game/SaticMesh/maschera.maschera")
    (Default|CallSoundStop)))

(event Custom|Left%20Stop
  (params (hitted :type Actor%20Object%20Reference))
  (bind _returnvalue (Transformation|GetActorLocation hitted))
  ;[1 1 1] Hit Left
  (if (== (Variables|Default|GetDirection) 3)
    (Variables|Default|Setmoving false)
    (Variables|Default|SetPosition (Math|Vector|MakeVector (.x _returnvalue) (- (.y _returnvalue) -1e+02) 5e+01))
    (Transformation|SetActorLocation (Variables|Default|GetMask) (Variables|Default|GetPosition) false false)
    (Variables|Default|SetEmitter%20position (Math|Vector|MakeVector (.X (Math|Vector|BreakVector (Variables|Default|GetPosition))) (+ (.Y (Math|Vector|BreakVector (Variables|Default|GetPosition))) -4e+01) (.Z (Math|Vector|BreakVector (Variables|Default|GetPosition)))))
    (Variables|Default|Setemitter%20rotation "0, 0,90.000000")
    ;[1 1 1] Play end movment effect
    (Effects|SpawnEmitteratLocation "/Game/Cascade/Hit.Hit" (Variables|Default|GetEmitter%20position) (Variables|Default|Getemitter%20rotation))
    (Components|StaticMesh|SetStaticMesh (Variables|/Game/Blueprints/Pawn/BP_Mask.BP_Mask_C|GetStaticMesh (Variables|Default|GetMask)) "/Game/SaticMesh/maschera.maschera")
    (Default|CallSoundStop)))

(event Custom|Right%20Stop
  (params (hitted :type Actor%20Object%20Reference))
  (bind _returnvalue (Transformation|GetActorLocation hitted))
  ;[1 1 1] Hit Right
  (if (== (Variables|Default|GetDirection) 2)
    (Variables|Default|Setmoving false)
    (Variables|Default|SetPosition (Math|Vector|MakeVector (.x _returnvalue) (- (.y _returnvalue) 1e+02) 5e+01))
    (Transformation|SetActorLocation (Variables|Default|GetMask) (Variables|Default|GetPosition) false false)
    (Variables|Default|SetEmitter%20position (Math|Vector|MakeVector (.X (Math|Vector|BreakVector (Variables|Default|GetPosition))) (+ (.Y (Math|Vector|BreakVector (Variables|Default|GetPosition))) 4e+01) (.Z (Math|Vector|BreakVector (Variables|Default|GetPosition)))))
    (Variables|Default|Setemitter%20rotation "0, 0,-90.000000")
    ;[1 1 1] Play end movment effect
    (Effects|SpawnEmitteratLocation "/Game/Cascade/Hit.Hit" (Variables|Default|GetEmitter%20position) (Variables|Default|Getemitter%20rotation))
    (Components|StaticMesh|SetStaticMesh (Variables|/Game/Blueprints/Pawn/BP_Mask.BP_Mask_C|GetStaticMesh (Variables|Default|GetMask)) "/Game/SaticMesh/maschera.maschera")
    (Default|CallSoundStop)))

(event Custom|Lose
  (bind _mask (Variables|Default|GetMask))
  ;[1 1 1] Obstacole's triggers
  (Utilities|FlowControl|DoOnce false
    (:Completed
      (Variables|Default|Setmoving false)
      (Rendering|SetVisibility (Variables|/Game/Blueprints/Pawn/BP_Mask.BP_Mask_C|GetStaticMesh _mask) false false)
      (Rendering|SetVisibility (Variables|/Game/Blueprints/Pawn/BP_Mask.BP_Mask_C|GetDestructible _mask) true false)
      (Class|RadialForceComponent|FireImpulse (Variables|/Game/Blueprints/Pawn/BP_Mask.BP_Mask_C|GetRadialForce _mask))
      (Variables|Default|Setdead true)
      (Default|CallDeath)
      (Utilities|FlowControl|Delay 0.5)
      (Variables|Default|SetLost true)
      (Variables|Default|SetbShowMouseCursor true))))

(event Custom|increment%20points
  ;[1 1 1] Increment points
  (Math|Integer|IncrementInt (Variables|Default|Getpoints)))

(event Custom|save
  ;[1 1 1] save the information at the end of the level
  (Variables|Default|SetEnd true)
  (Variables|Default|Setmoving true)
  (Variables|Default|SetbShowMouseCursor true)
  (switch int (- (Variables|/Game/Blueprints/BP_Var.BP_Var_C|GetLevel (Variables|Default|GetStore)) 1)
    (:0
      (|SAVE1))
    (:1
      (|CollapseGraph_2))
    (:2
      (|CollapseGraph_1))
    (:3
      (|CollapseGraph_0))))

(event EventBeginPlay
  ;[1 1 1] Inizializzazione
  (Variables|Default|Setdead false)
  (bind _asbp_var (Utilities|Casting|CastToBP_Var (Game|GetGameInstance)))
  (Variables|Default|SetStore _asbp_var)
  (bind _outactors (Actor|GetAllActorswithTag "wall"))
  (Variables|Default|SetWalls _outactors)
  (bind _asbp_mask (Utilities|Casting|CastToBP_Mask (Game|Player|GetPlayerPawn 0)))
  (bind _output_get (Variables|Default|SetMask _asbp_mask))
  (Variables|Default|SetPosition (Transformation|GetActorLocation _output_get))
  (switch int (Variables|/Game/Blueprints/BP_Var.BP_Var_C|GetLevel (Variables|Default|GetStore))
    (:Default
      _)
    (:0
      (Variables|Default|SettotalPoint 67.0))
    (:1
      (Variables|Default|SettotalPoint 146.0))
    (:2
      (Variables|Default|SettotalPoint 76.0))
    (:3
      (Variables|Default|SettotalPoint 228.0)))
  ;[1 1 1] save the information at the end of the level
  (bind _returnvalue (Actor|GetActorOfClass "/Game/Blueprints/Actor/Walls/BP_Base.BP_Base_C"))
  (EventDispatchers|BindEventtoEnd _returnvalue (delegate Custom|save))
  ;[1 1 1] Increment points
  (bind _outactors_2 (Actor|GetAllActorsOfClass "/Game/Blueprints/Actor/Collectable/BP_Points.BP_Points_C"))
  (for _array_element _outactors_2
    (EventDispatchers|BindEventtoDestroyed _array_element (delegate Custom|increment%20points)))
  ;[1 1 1] Obstacole's triggers
  (bind _outactors_3 (Actor|GetAllActorsOfClass "/Game/Blueprints/Actor/Obstacoles/BP_3Spike.BP_3Spike_C"))
  (for _array_element_2 _outactors_3
    (EventDispatchers|BindEventtoLoseby3Spike _array_element_2 (delegate Custom|Lose)))
  (bind _outactors_4 (Actor|GetAllActorsOfClass "/Game/Blueprints/Actor/Obstacoles/BP_2Spike.BP_2Spike_C"))
  (for _array_element_3 _outactors_4
    (EventDispatchers|BindEventtoLoseby2Spike _array_element_3 (delegate Custom|Lose)))
  (bind _outactors_5 (Actor|GetAllActorsOfClass "/Game/Blueprints/Actor/Obstacoles/BP_Spike.BP_Spike_C"))
  (for _array_element_4 _outactors_5
    (EventDispatchers|BindEventtoLosebySpike _array_element_4 (delegate Custom|Lose)))
  (bind _outactors_6 (Actor|GetAllActorsOfClass "/Game/Blueprints/Actor/Obstacoles/BP_TriggerSpike.BP_TriggerSpike_C"))
  (for _array_element_5 _outactors_6
    (EventDispatchers|BindEventtoLose _array_element_5 (delegate Custom|Lose)))
  (bind _outactors_7 (Actor|GetAllActorsOfClass "/Game/Blueprints/Actor/Obstacoles/BP_Bat.BP_Bat_C"))
  (for _array_element_6 _outactors_7
    (EventDispatchers|BindEventtoLosebyBat _array_element_6 (delegate Custom|Lose)))
  (bind _outactors_8 (Actor|GetAllActorsOfClass "/Game/Blueprints/Actor/Obstacoles/BP_StartSpike.BP_StartSpike_C"))
  (for _array_element_7 _outactors_8
    (EventDispatchers|BindEventtoLosebySpike _array_element_7 (delegate Custom|Lose)))
  ;[1 1 1] Hit Front
  (EventDispatchers|BindEventtoFrontStop (Variables|Default|GetMask) (delegate Custom|Stop%20Front))
  ;[1 1 1] Hit Back
  (EventDispatchers|BindEventtoBackStop (Variables|Default|GetMask) (delegate Custom|Stop%20Back))
  ;[1 1 1] Hit Left
  (EventDispatchers|BindEventtoLeftStop (Variables|Default|GetMask) (delegate Custom|Left%20Stop))
  ;[1 1 1] Hit Right
  (EventDispatchers|BindEventtoRightStop (Variables|Default|GetMask) (delegate Custom|Right%20Stop)))

(event EventTick
  (params (DeltaSeconds :type Float%20%28single-precision%29))
  ;[1 1 1] traslazione
  (if (not (Variables|Default|GetLost))
    (if (not (Variables|Default|GetEnd))
      (if (not (Variables|Default|GetPausa))
        (if (Variables|Default|Getmoving)
          (switch int (Variables|Default|GetDirection)
            (:0
              (Variables|Default|SetPosition (Math|Vector|MakeVector (+ (.x (Variables|Default|GetPosition)) (* 1 (* (Variables|Default|GetSpeed) DeltaSeconds))) (.y (Variables|Default|GetPosition)) (.z (Variables|Default|GetPosition)))))
            (:1
              (Variables|Default|SetPosition (Math|Vector|MakeVector (+ (.x (Variables|Default|GetPosition)) (* -1 (* (Variables|Default|GetSpeed) DeltaSeconds))) (.y (Variables|Default|GetPosition)) (.z (Variables|Default|GetPosition)))))
            (:2
              (Variables|Default|SetPosition (Math|Vector|MakeVector (.x (Variables|Default|GetPosition)) (+ (.y (Variables|Default|GetPosition)) (* 1 (* (Variables|Default|GetSpeed) DeltaSeconds))) (.z (Variables|Default|GetPosition)))))
            (:3
              (Variables|Default|SetPosition (Math|Vector|MakeVector (.x (Variables|Default|GetPosition)) (+ (.y (Variables|Default|GetPosition)) (* -1 (* (Variables|Default|GetSpeed) DeltaSeconds))) (.z (Variables|Default|GetPosition))))))
          (Transformation|SetActorLocation (Variables|Default|GetMask) (Variables|Default|GetPosition) false false)
          (Effects|SpawnEmitteratLocation "/Game/Cascade/Scia.Scia" (Variables|Default|GetPosition) (Variables|Default|GetRotation)))))))

(event Input|ActionEvents|InputActionForward
  (params (Key :type Key%20Structure :default "None"))
  ;[1 1 1] movment
  (:Pressed
    (if (not (Variables|Default|GetPausa))
      (if (not (Variables|Default|Getmoving))
        (Variables|Default|SetDirection 0)
        (Variables|Default|SetRotation "-30.000000,-90.000000,-90.000000")
        (if (Variables|Default|Getdead)
          _
          (else
            _))
        (for _array_element (Variables|Default|GetWalls)
          (if (Math|Vector|Equal(Vector) (+ (Transformation|GetActorLocation _array_element) "-100.000000,0.000000,50.000000") (Transformation|GetActorLocation (Variables|Default|GetMask)) 1e+01)
            (Variables|Default|SetcanMove false)))
        (if (Variables|Default|GetcanMove)
          (Variables|Default|Setmoving true)
          (Default|CallMove)
          (Components|StaticMesh|SetStaticMesh (Variables|/Game/Blueprints/Pawn/BP_Mask.BP_Mask_C|GetStaticMesh (Variables|Default|GetMask)) "/Game/SaticMesh/sphere.sphere")
          (else
            (Variables|Default|SetcanMove true)))))))

(event Input|ActionEvents|InputActionBackward
  (params (Key :type Key%20Structure :default "None"))
  ;[1 1 1] movment
  (:Pressed
    (if (not (Variables|Default|GetPausa))
      (if (not (Variables|Default|Getmoving))
        (Variables|Default|SetDirection 1)
        (Variables|Default|SetRotation "-30.000000,90.000000,-90.000000")
        (if (not (Variables|Default|Getdead))
          (for _array_element (Variables|Default|GetWalls)
            (if (Math|Vector|Equal(Vector) (+ (Transformation|GetActorLocation _array_element) "100.000000,0.000000,50.000000") (Transformation|GetActorLocation (Variables|Default|GetMask)) 1e+01)
              (Variables|Default|SetcanMove false)))
          (if (Variables|Default|GetcanMove)
            (Variables|Default|Setmoving true)
            (Default|CallMove)
            (Components|StaticMesh|SetStaticMesh (Variables|/Game/Blueprints/Pawn/BP_Mask.BP_Mask_C|GetStaticMesh (Variables|Default|GetMask)) "/Game/SaticMesh/sphere.sphere")
            (else
              (Variables|Default|SetcanMove true))))))))

(event Input|ActionEvents|InputActionLeft
  (params (Key :type Key%20Structure :default "None"))
  ;[1 1 1] movment
  (:Pressed
    (if (not (Variables|Default|GetPausa))
      (if (not (Variables|Default|Getmoving))
        (Variables|Default|SetDirection 3)
        (Variables|Default|SetRotation "-30.000000,180.000000,-90.000000")
        (if (not (Variables|Default|Getdead))
          (for _array_element (Variables|Default|GetWalls)
            (if (Math|Vector|Equal(Vector) (+ (Transformation|GetActorLocation _array_element) "0.000000,100.000000,50.000000") (Transformation|GetActorLocation (Variables|Default|GetMask)) 1e+01)
              (Variables|Default|SetcanMove false)))
          (if (Variables|Default|GetcanMove)
            (Variables|Default|Setmoving true)
            (Default|CallMove)
            (Components|StaticMesh|SetStaticMesh (Variables|/Game/Blueprints/Pawn/BP_Mask.BP_Mask_C|GetStaticMesh (Variables|Default|GetMask)) "/Game/SaticMesh/sphere.sphere")
            (else
              (Variables|Default|SetcanMove true))))))))

(event Input|ActionEvents|InputActionrestart
  (params (Key :type Key%20Structure :default "None"))
  (bind _store (Variables|Default|GetStore))
  (:Pressed
    (if (not (or (Variables|/Game/Blueprints/BP_Var.BP_Var_C|GetMainMenu _store) (Variables|/Game/Blueprints/BP_Var.BP_Var_C|GetEndMenu _store)))
      (switch int (Variables|/Game/Blueprints/BP_Var.BP_Var_C|GetLevel _store)
        (:0
          (Game|OpenLevel(byName) "1stLevel"))
        (:1
          (Game|OpenLevel(byName) "2ndLevel"))
        (:2
          (Game|OpenLevel(byName) "3tdLevel"))
        (:3
          (Game|OpenLevel(byName) "4thLevel"))))))

(event Input|ActionEvents|InputActionclose
  (params (Key :type Key%20Structure :default "None"))
  ;[1 1 1] main menu
  (:Pressed
    (Game|OpenLevel(byName) "MainMenu")))

(event Input|ActionEvents|InputActionPause
  (params (Key :type Key%20Structure :default "None"))
  ;[1 1 1] pause
  (:Pressed
    (Variables|Default|SetPausa (not (Variables|Default|GetPausa)))
    (Variables|Default|SetbShowMouseCursor (not (Variables|Default|GetbShowMouseCursor)))))

(event Input|ActionEvents|InputActionRight
  (params (Key :type Key%20Structure :default "None"))
  ;[1 1 1] movment
  (:Pressed
    (if (not (Variables|Default|GetPausa))
      (if (not (Variables|Default|Getmoving))
        (Variables|Default|SetDirection 2)
        (Variables|Default|SetRotation "-30.000000,0.000000,-90.000000")
        (if (not (Variables|Default|Getdead))
          (for _array_element (Variables|Default|GetWalls)
            (if (Math|Vector|Equal(Vector) (+ (Transformation|GetActorLocation _array_element) "0.000000,-100.000000,50.000000") (Transformation|GetActorLocation (Variables|Default|GetMask)) 1e+01)
              (Variables|Default|SetcanMove false)))
          (if (Variables|Default|GetcanMove)
            (Variables|Default|Setmoving true)
            (Default|CallMove)
            (Components|StaticMesh|SetStaticMesh (Variables|/Game/Blueprints/Pawn/BP_Mask.BP_Mask_C|GetStaticMesh (Variables|Default|GetMask)) "/Game/SaticMesh/sphere.sphere")
            (else
              (Variables|Default|SetcanMove true))))))))

(fn ConstructionScript)