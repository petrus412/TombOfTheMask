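; BP_Mask is the mask pawn, which detects blocking contacts on four sides and can trigger a loss on spikes.
; Each Tick it rotates its mesh to the Rotation held by BP_PlayerController, cached at BeginPlay.
; Front, back, left and right overlap components ignore points, stars and other masks; any other actor fires that side's Stop dispatcher.
; Touching a BP_TriggerSpike that is Out also calls its Lose dispatcher first.
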(event OnComponentBeginOverlap(DirectionFront)
  (params (OverlappedComponent :type Primitive%20Component%20Object%20Reference) (OtherActor :type Actor%20Object%20Reference) (OtherComp :type Primitive%20Component%20Object%20Reference) (OtherBodyIndex :type Integer) (bFromSweep :type Boolean) (SweepResult :type Hit%20Result%20Structure%20%28by%20ref%29))
  (Utilities|Casting|CastToBP_Points OtherActor
    (:CastFailed
      (Utilities|Casting|CastToBP_star OtherActor
        (:CastFailed
          (Utilities|Casting|CastToBP_Mask OtherActor
            (:CastFailed
              (bind _asbp_trigger_spike (Utilities|Casting|CastToBP_TriggerSpike OtherActor)
                (:then
                  (if (Variables|/Game/Blueprints/Actor/Obstacoles/BP_TriggerSpike.BP_TriggerSpike_C|GetOut _asbp_trigger_spike)
                    (Default|CallLose _asbp_trigger_spike)))
                (:CastFailed
                  _))
              (Default|CallFrontStop))))))))

(event OnComponentBeginOverlap(DirectionBack)
  (params (OverlappedComponent :type Primitive%20Component%20Object%20Reference) (OtherActor :type Actor%20Object%20Reference) (OtherComp :type Primitive%20Component%20Object%20Reference) (OtherBodyIndex :type Integer) (bFromSweep :type Boolean) (SweepResult :type Hit%20Result%20Structure%20%28by%20ref%29))
  (Utilities|Casting|CastToBP_Points OtherActor
    (:CastFailed
      (Utilities|Casting|CastToBP_star OtherActor
        (:CastFailed
          (Utilities|Casting|CastToBP_Mask OtherActor
            (:CastFailed
              (bind _asbp_trigger_spike (Utilities|Casting|CastToBP_TriggerSpike OtherActor)
                (:then
                  (if (Variables|/Game/Blueprints/Actor/Obstacoles/BP_TriggerSpike.BP_TriggerSpike_C|GetOut _asbp_trigger_spike)
                    (Default|CallLose _asbp_trigger_spike)))
                (:CastFailed
                  _))
              (Default|CallBackStop))))))))

(event OnComponentBeginOverlap(DirectionLeft)
  (params (OverlappedComponent :type Primitive%20Component%20Object%20Reference) (OtherActor :type Actor%20Object%20Reference) (OtherComp :type Primitive%20Component%20Object%20Reference) (OtherBodyIndex :type Integer) (bFromSweep :type Boolean) (SweepResult :type Hit%20Result%20Structure%20%28by%20ref%29))
  (Utilities|Casting|CastToBP_Points OtherActor
    (:CastFailed
      (Utilities|Casting|CastToBP_star OtherActor
        (:CastFailed
          (Utilities|Casting|CastToBP_Mask OtherActor
            (:CastFailed
              (bind _asbp_trigger_spike (Utilities|Casting|CastToBP_TriggerSpike OtherActor)
                (:then
                  (if (Variables|/Game/Blueprints/Actor/Obstacoles/BP_TriggerSpike.BP_TriggerSpike_C|GetOut _asbp_trigger_spike)
                    (Default|CallLose _asbp_trigger_spike)))
                (:CastFailed
                  _))
              (Default|CallLeftStop))))))))

(event OnComponentBeginOverlap(DirectionRight)
  (params (OverlappedComponent :type Primitive%20Component%20Object%20Reference) (OtherActor :type Actor%20Object%20Reference) (OtherComp :type Primitive%20Component%20Object%20Reference) (OtherBodyIndex :type Integer) (bFromSweep :type Boolean) (SweepResult :type Hit%20Result%20Structure%20%28by%20ref%29))
  (Utilities|Casting|CastToBP_Points OtherActor
    (:CastFailed
      (Utilities|Casting|CastToBP_star OtherActor
        (:CastFailed
          (Utilities|Casting|CastToBP_Mask OtherActor
            (:CastFailed
              (bind _asbp_trigger_spike (Utilities|Casting|CastToBP_TriggerSpike OtherActor)
                (:then
                  (if (Variables|/Game/Blueprints/Actor/Obstacoles/BP_TriggerSpike.BP_TriggerSpike_C|GetOut _asbp_trigger_spike)
                    (Default|CallLose _asbp_trigger_spike)))
                (:CastFailed
                  _))
              (Default|CallRightStop))))))))

(event EventBeginPlay
  (bind _asbp_player_controller (Utilities|Casting|CastToBP_PlayerController (Game|GetPlayerController 0)))
  (Variables|Default|SetPlayerController _asbp_player_controller))

(event EventTick
  (params (DeltaSeconds :type Float%20%28single-precision%29))
  (Transformation|SetRelativeRotation (Variables|Default|GetStaticMesh) (Variables|/Game/Blueprints/Pawn/BP_PlayerController.BP_PlayerController_C|GetRotation (Variables|Default|GetPlayerController)) false false))

(fn ConstructionScript)